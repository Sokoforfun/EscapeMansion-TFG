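; BP_PuertaSalida is the exit door that ends the game once the player has collected at least three keys.
; Box overlap shows a prompt widget and enables input on the actor, and leaving reverses both, with no check on the overlapping actor.
; Pressing E reads CantidadLlaves from the player character, then either opens WBP_FinJuego with the mouse cursor or briefly shows a WBP_Aviso warning.
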(event OnComponentBeginOverlap(Box)
  (params (OverlappedComponent :type Primitive%20Component%20Object%20Reference) (OtherActor :type Actor%20Object%20Reference) (OtherComp :type Primitive%20Component%20Object%20Reference) (OtherBodyIndex :type Integer) (bFromSweep :type Boolean) (SweepResult :type Hit%20Result%20Structure%20%28by%20ref%29))
  (Rendering|SetVisibility (Variables|Default|GetWidget) true false)
  (Input|EnableInput (Game|GetPlayerController 0)))

(event OnComponentEndOverlap(Box)
  (params (OverlappedComponent :type Primitive%20Component%20Object%20Reference) (OtherActor :type Actor%20Object%20Reference) (OtherComp :type Primitive%20Component%20Object%20Reference) (OtherBodyIndex :type Integer))
  (Rendering|SetVisibility (Variables|Default|GetWidget) false false)
  (Input|DisableInput (Game|GetPlayerController 0)))

(event EventBeginPlay)

(event Collision|EventActorBeginOverlap
  (params (OtherActor :type Actor%20Object%20Reference)))

(event EventTick
  (params (DeltaSeconds :type Float%20%28single-precision%29)))

(event Input|KeyboardEvents|E
  (params (Key :type Key%20Structure))
  (:Pressed
    (bind _asbp_third_person_character (Utilities|Casting|CastToBP_ThirdPersonCharacter (Game|GetPlayerCharacter 0)))
    (if (>= (Variables|/Game/ThirdPerson/Blueprints/BP_ThirdPersonCharacter.BP_ThirdPersonCharacter_C|GetCantidadLlaves _asbp_third_person_character) 3)
      (bind _returnvalue (UserInterface|CreateWidget "/Game/02_Blueprints/FinalDelJuego/WBP_FinJuego.WBP_FinJuego_C"))
      (UserInterface|Viewport|AddtoViewport _returnvalue 0)
      (Variables|/Script/Engine.PlayerController|SetbShowMouseCursor (Game|GetPlayerController 0) true)
      (else
        (bind _returnvalue_2 (UserInterface|CreateWidget "/Game/02_Blueprints/IconosYAvisos/WBP_Aviso.WBP_Aviso_C"))
        (bind _output_get (Variables|Default|SetWidget%20Aviso _returnvalue_2))
        (Rendering|Components|TextRender|SetText (Variables|/Game/02_Blueprints/IconosYAvisos/WBP_Aviso.WBP_Aviso_C|GetTxt_Mensaje _output_get) "Necesito 3 llaves para abrir esta puerta...")
        (UserInterface|Viewport|AddtoViewport _output_get 0)
        (Utilities|FlowControl|Delay 3.0)
        (Widget|RemovefromParent _output_get)))))

(fn ConstructionScript)