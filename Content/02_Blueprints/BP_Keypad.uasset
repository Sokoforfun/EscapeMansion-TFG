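; BP_Keypad is an interactable keypad actor that opens a code-entry widget linked to a selected door.
; Overlapping BoxColision shows a prompt widget component and enables input; leaving hides it and disables input.
; Pressing E toggles WBP_Keypad, passing PuertaSeleccionada and switching input mode and mouse cursor.
; A success handler calls OnCorrectCode, but its binding to the widget's OnExito is never executed.
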(event OnComponentBeginOverlap(BoxColision)
  (params (OverlappedComponent :type Primitive%20Component%20Object%20Reference) (OtherActor :type Actor%20Object%20Reference) (OtherComp :type Primitive%20Component%20Object%20Reference) (OtherBodyIndex :type Integer) (bFromSweep :type Boolean) (SweepResult :type Hit%20Result%20Structure%20%28by%20ref%29))
  (Rendering|SetVisibility (Variables|Default|GetWidget) true false)
  (Input|EnableInput (Game|GetPlayerController 0))
  (Development|PrintString "ESTOY DENTRO")
  (Input|EnableInput (Game|GetPlayerController 0)))

(event OnComponentEndOverlap(BoxColision)
  (params (OverlappedComponent :type Primitive%20Component%20Object%20Reference) (OtherActor :type Actor%20Object%20Reference) (OtherComp :type Primitive%20Component%20Object%20Reference) (OtherBodyIndex :type Integer))
  (Rendering|SetVisibility (Variables|Default|GetWidget) false false)
  (Input|DisableInput (Game|GetPlayerController 0) 0)
  (Development|PrintString "HE SALIDOO")
  (Input|DisableInput (Game|GetPlayerController 0)))

(event Custom|OnExito_Event
  (Default|CallOnCorrectCode))

(event Collision|EventActorBeginOverlap
  (params (OtherActor :type Actor%20Object%20Reference)))

(event EventTick
  (params (DeltaSeconds :type Float%20%28single-precision%29)))

(event Input|KeyboardEvents|E
  (params (Key :type Key%20Structure))
  (bind _returnvalue (Game|GetPlayerController 0))
  (:Pressed
    (Utilities|IsValid (Variables|Default|GetKeypadWidgetRef)
      (:Is%20Valid
        (Widget|RemovefromParent (Variables|Default|GetKeypadWidgetRef))
        (Variables|Default|SetKeypadWidgetRef 0)
        (Input|SetInputModeGameOnly _returnvalue false)
        (Variables|/Script/Engine.PlayerController|SetbShowMouseCursor _returnvalue false))
      (:Is%20Not%20Valid
        (Development|PrintString "PULSA LA E")
        (bind _returnvalue_2 (UserInterface|CreateWidget "/Game/02_Blueprints/WBP_Keypad.WBP_Keypad_C" _returnvalue (Variables|Default|GetPuertaSeleccionada)))
        (Variables|Default|SetKeypadWidgetRef _returnvalue_2)
        (UserInterface|Viewport|AddtoViewport _returnvalue_2 0)
        (Development|PrintString "WIDGET CREADO")
        (Input|SetInputModeGameandUI _returnvalue _returnvalue_2 "DoNotLock" true false)
        (Variables|/Script/Engine.PlayerController|SetbShowMouseCursor _returnvalue true)))))

(fn ConstructionScript)