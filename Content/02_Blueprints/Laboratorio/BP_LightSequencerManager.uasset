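; Manager actor in the laboratory that flashes an array of lights one after another, each a set number of times, as a repeating blink pattern.
; On BeginPlay it hides every PointLight, then blinks each in turn using its count from Patron and the VelocidadParpadeo delay.
; Custom events call each other around Delays to advance blinks and lights, restarting after a short pause once the array ends.
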(event Custom|Iniciar%20Secuencia
  (Variables|Default|SetBombillaPorLaQueVamos 0)
  (Variables|Default|SetContadorParpadeos 0)
  (for _array_element (Variables|Default|GetLucesArray)
    (Rendering|SetVisibility (Actor|GetComponentbyClass _array_element "/Script/Engine.PointLightComponent") false false))
  (CallFunction|ProcesarSiguienteLuz))

(event Custom|ProcesarSiguienteLuz
  (if (>= (Variables|Default|GetBombillaPorLaQueVamos) (Utilities|Array|Length (Variables|Default|GetLucesArray)))
    (Utilities|FlowControl|Delay 2.0)
    (CallFunction|IniciarSecuencia)
    (else
      (Variables|Default|SetContadorParpadeos 0)
      (CallFunction|ParpadearLuzActual))))

(event Custom|ParpadearLuzActual
  (if (>= (Variables|Default|GetContadorParpadeos) (Utilities|Array|Get(acopy) (Variables|Default|GetPatron) (Variables|Default|GetBombillaPorLaQueVamos)))
    (Rendering|SetVisibility (Variables|Default|GetDefaultSceneRoot) false false)
    (Math|Integer|IncrementInt (Variables|Default|GetBombillaPorLaQueVamos)
      (:%20%20
        (CallFunction|ProcesarSiguienteLuz)))
    (else
      (Rendering|SetVisibility (Actor|GetComponentbyClass (Utilities|Array|Get(acopy) (Variables|Default|GetLucesArray) (Variables|Default|GetBombillaPorLaQueVamos)) "/Script/Engine.PointLightComponent") true false)
      (Utilities|FlowControl|Delay (Variables|Default|GetVelocidadParpadeo))
      (Rendering|SetVisibility (Actor|GetComponentbyClass (Utilities|Array|Get(acopy) (Variables|Default|GetLucesArray) (Variables|Default|GetBombillaPorLaQueVamos)) "/Script/Engine.PointLightComponent") false false)
      (Utilities|FlowControl|Delay (Variables|Default|GetVelocidadParpadeo))
      (Math|Integer|IncrementInt (Variables|Default|GetContadorParpadeos)
        (:%20%20
          (CallFunction|ParpadearLuzActual))))))

(event EventBeginPlay
  (CallFunction|IniciarSecuencia))

(event Collision|EventActorBeginOverlap
  (params (OtherActor :type Actor%20Object%20Reference)))

(event EventTick
  (params (DeltaSeconds :type Float%20%28single-precision%29)))

(fn ConstructionScript)