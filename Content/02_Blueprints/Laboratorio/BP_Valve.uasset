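; Clickable valve actor that plays a sound and rotates its mesh a quarter turn on each interaction.
; Clicking calls Interact, while OnValveInteracted starts a timeline that lerps the mesh yaw from its current value to 90 degrees further.
; A box overlap shows the widget and enables input, and leaving it hides the widget and disables input.
; The sound is positioned using the mesh's relative location, not its world location.
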(event OnComponentBeginOverlap(Box)
  (params (OverlappedComponent :type Primitive%20Component%20Object%20Reference) (OtherActor :type Actor%20Object%20Reference) (OtherComp :type Primitive%20Component%20Object%20Reference) (OtherBodyIndex :type Integer) (bFromSweep :type Boolean) (SweepResult :type Hit%20Result%20Structure%20%28by%20ref%29))
  (Rendering|SetVisibility (Variables|Default|GetWidget) true false)
  (Input|EnableInput (Game|GetPlayerController 0)))

(event OnComponentEndOverlap(Box)
  (params (OverlappedComponent :type Primitive%20Component%20Object%20Reference) (OtherActor :type Actor%20Object%20Reference) (OtherComp :type Primitive%20Component%20Object%20Reference) (OtherBodyIndex :type Integer))
  (Rendering|SetVisibility (Variables|Default|GetWidget) false false)
  (Input|DisableInput (Game|GetPlayerController 0) 0))

(event Collision|EventActorBeginOverlap
  (params (OtherActor :type Actor%20Object%20Reference)))

(event EventTick
  (params (DeltaSeconds :type Float%20%28single-precision%29)))

(event MouseInput|EventActorOnClicked
  (params (ButtonPressed :type Key%20Structure))
  (Class|ValveBase|Interact))

(event EventOnValveInteracted
  (params (NewAngle :type Float%20%28single-precision%29))
  (Variables|Default|SetRotacionInicial (.yaw (Variables|/Script/Engine.SceneComponent|GetRelativeRotation (Variables|Default|GetValveMesh))))
  (Audio|PlaySoundatLocation "/Game/01_Audio/Sound_Valve.Sound_Valve" (Variables|/Script/Engine.SceneComponent|GetRelativeLocation (Variables|Default|GetValveMesh)) "0, 0, 0" 1.0 1.0 0.0 0 0 0 0)
  (bind _giro (Timeline|GiroTimeLine PlayFromStart)
    (:Update
      (Transformation|SetRelativeRotation (Variables|Default|GetValveMesh) (Math|Rotator|MakeRotator 0.0 0.0 (Math|Float|Lerp (Variables|Default|GetRotacionInicial) (- (Variables|Default|GetRotacionInicial) -9e+01) _giro)) false false))))

(fn ConstructionScript)