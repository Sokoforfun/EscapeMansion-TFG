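; Valve puzzle checker actor that spawns a laboratory key (BP_LaboratorioLlave) once all its valves are correct.
; On BeginPlay it binds to the rotation delegate of every valve in ValvulasArray, apparently to drive VerificarCorrecto.
; That check stops at the first incorrect valve, otherwise spawns the key at the Spawnpoint transform, with no guard against repeat spawns.
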(event Custom|VerificarCorrecto
  (Development|PrintString "Verificando Valvula")
  (Variables|Default|SetTodoCorrecto true)
  (bind _array_element (Utilities|Array|ForEachLoopwithBreak (Variables|Default|GetValvulasArray) :!label _label)
    (:LoopBody
      (bind _returnvalue (Class|ValveBase|IsCorrect _array_element))
      (if (not _returnvalue)
        (Variables|Default|SetTodoCorrecto false)
        (goto _label Break)))
    (:Completed
      (if (Variables|Default|GetTodoCorrecto)
        (Game|SpawnActorfromClass "/Game/HUD/Pickups/BP_LaboratorioLlave.BP_LaboratorioLlave_C" (Transformation|GetWorldTransform (Variables|Default|GetSpawnpoint)) "Undefined" "MultiplyWithRoot" 0 0)))))

(event EventBeginPlay
  (for _array_element (Variables|Default|GetValvulasArray)
    (EventDispatchers|BindEventtoOnValveRotatedDelegate _array_element (EventDispatchers|CreateEvent :!event Custom|VerificarCorrecto))))

(event Collision|EventActorBeginOverlap
  (params (OtherActor :type Actor%20Object%20Reference)))

(event EventTick
  (params (DeltaSeconds :type Float%20%28single-precision%29)))

(fn ConstructionScript)