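; BP_Puerta_Lab is a lab door that slides open when either custom event, PuertaAbrir or ABRIR_YA, is called.
; Both events share one chain that plays a button-click sound, stores the door's current relative location and restarts a timeline.
; The timeline lerps the door along relative X from that stored position, printing a debug message on each update.
; The Blueprint has no closing logic.
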(event Custom|ABRIR_YA
  (bind _puerta (Variables|Default|GetPuerta))
  (Audio|PlaySound2D "/Engine/VREditor/Sounds/UI/Click_on_Button.Click_on_Button" 1.0 1.0 0.0 0 0)
  (bind _output_get (Variables|Default|SetPosInicial (Variables|/Script/Engine.SceneComponent|GetRelativeLocation _puerta)))
  (bind _newtrack_0 (Timeline|AnimacionPuerta PlayFromStart)
    (:Update
      (Development|PrintString "MOVIENDO")
      (Transformation|SetRelativeLocation _puerta (Math|Vector|Lerp(Vector) _output_get (+ _output_get "8000.000000,0.000000,0.000000") _newtrack_0) false false))))

(event EventBeginPlay)

(event Collision|EventActorBeginOverlap
  (params (OtherActor :type Actor%20Object%20Reference)))

(event EventTick
  (params (DeltaSeconds :type Float%20%28single-precision%29)))

(event EventPuertaAbrir
  (bind _puerta (Variables|Default|GetPuerta))
  (Audio|PlaySound2D "/Engine/VREditor/Sounds/UI/Click_on_Button.Click_on_Button" 1.0 1.0 0.0 0 0)
  (bind _output_get (Variables|Default|SetPosInicial (Variables|/Script/Engine.SceneComponent|GetRelativeLocation _puerta)))
  (bind _newtrack_0 (Timeline|AnimacionPuerta PlayFromStart)
    (:Update
      (Development|PrintString "MOVIENDO")
      (Transformation|SetRelativeLocation _puerta (Math|Vector|Lerp(Vector) _output_get (+ _output_get "8000.000000,0.000000,0.000000") _newtrack_0) false false))))

(fn ConstructionScript)