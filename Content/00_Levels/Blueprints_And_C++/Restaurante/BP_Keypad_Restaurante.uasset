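; Interactable keypad for the restaurant level that opens a code-entry widget linked to a selected door.
; Its box collision shows a widget component and enables player input while overlapped.
; Pressing E toggles the keypad UI, passing it the door reference and switching input mode and mouse cursor.
; An OnCorrectCode dispatcher is meant to relay the keypad's success event, but that binding is unconnected and never runs.
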(event OnComponentBeginOverlap(BoxColision)
  (params (OverlappedComponent :type Primitive%20Component%20Object%20Reference) (OtherActor :type Actor%20Object%20Reference) (OtherComp :type Primitive%20Component%20Object%20Reference) (OtherBodyIndex :type Integer) (bFromSweep :type Boolean) (SweepResult :type Hit%20Result%20Structure%20%28by%20ref%29))
  (Rendering|SetVisibility (Variables|Default|GetWidget) true false)
  (Input|EnableInput (Game|GetPlayerController 0)))

(event OnComponentEndOverlap(BoxColision)
  (params (OverlappedComponent :type Primitive%20Component%20Object%20Reference) (OtherActor :type Actor%20Object%20Reference) (OtherComp :type Primitive%20Component%20Object%20Reference) (OtherBodyIndex :type Integer))
  (Rendering|SetVisibility (Variables|Default|GetWidget) false false)
  (Input|DisableInput (Game|GetPlayerController 0)))

(event Custom|OnExito_Event
  (Default|CallOnCorrectCode))

(event Collision|EventActorBeginOverlap
  (params (OtherActor :type Actor%20Object%20Reference)))

(event EventTick
  (params (DeltaSeconds :type Float%20%28single-precision%29)))

(event Input|KeyboardEvents|E
  (params (Key :type Key%20Structure :default "None"))
  (bind _returnvalue (Game|GetPlayerController 0))
  (:Pressed
    (Utilities|IsValid (Variables|Default|GetRestaurantWidgetRef)
      (:Is%20Valid
        (Widget|RemovefromParent (Variables|Default|GetRestaurantWidgetRef))
        (Input|SetInputModeGameOnly _returnvalue false)
        (Variables|/Script/Engine.PlayerController|SetbShowMouseCursor _returnvalue false)
        (Variables|Default|SetRestaurantWidgetRef 0))
      (:Is%20Not%20Valid
        (Development|PrintString "PULSA LA E")
        (bind _returnvalue_2 (UserInterface|CreateWidget "/Game/00_Levels/Blueprints_And_C++/Restaurante/WBP_Keypad_Restaurante.WBP_Keypad_Restaurante_C" _returnvalue (Variables|Default|GetPuertaSeleccionada)))
        (Variables|Default|SetRestaurantWidgetRef _returnvalue_2)
        (UserInterface|Viewport|AddtoViewport _returnvalue_2 0)
        (Development|PrintString "WIDGET CREADO")
        (Input|SetInputModeGameandUI _returnvalue _returnvalue_2 "DoNotLock" true false)
        (Variables|/Script/Engine.PlayerController|SetbShowMouseCursor _returnvalue true)))))

(fn ConstructionScript)