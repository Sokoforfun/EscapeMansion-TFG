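; BP_Robot is an interactable restaurant robot that travels along a spline route once it has a battery.
; Its box overlap toggles a prompt widget and player input.
; Interactuar starts the trip if powered, copies the battery flag from the third-person character, or prints a no-energy message.
; A timeline maps progress to spline distance for location and rotation; its moving-state guard is cleared on finish but never set here.
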(event OnComponentBeginOverlap(Box)
  (params (OverlappedComponent :type Primitive%20Component%20Object%20Reference) (OtherActor :type Actor%20Object%20Reference) (OtherComp :type Primitive%20Component%20Object%20Reference) (OtherBodyIndex :type Integer) (bFromSweep :type Boolean) (SweepResult :type Hit%20Result%20Structure%20%28by%20ref%29))
  (Rendering|SetVisibility (Variables|Default|GetWidget) true false)
  (Input|EnableInput (Game|GetPlayerController 0)))

(event OnComponentEndOverlap(Box)
  (params (OverlappedComponent :type Primitive%20Component%20Object%20Reference) (OtherActor :type Actor%20Object%20Reference) (OtherComp :type Primitive%20Component%20Object%20Reference) (OtherBodyIndex :type Integer))
  (Rendering|SetVisibility (Variables|Default|GetWidget) false false)
  (Input|DisableInput (Game|GetPlayerController 0)))

(event Custom|IniciarRecorrido
  (bind _rutaaseguir (Variables|Default|GetRutaASeguir))
  (bind _spline (Variables|/Game/00_Levels/Blueprints_And_C++/Restaurante/BP_RutaRobot.BP_RutaRobot_C|GetSpline _rutaaseguir))
  (bind _recorridorobot (Timeline|MovimientoRobot PlayFromStart)
    (:Update
      (Transformation|SetActorLocationAndRotation (Spline|GetLocationatDistanceAlongSpline _spline (* _recorridorobot (Spline|GetSplineLength _spline)) "World") (Spline|GetRotationatDistanceAlongSpline _spline (* _recorridorobot (Spline|GetSplineLength _spline)) "World")))
    (:Finished
      (Variables|Default|SetEstaMoviendose false))))

(event EventBeginPlay)

(event Collision|EventActorBeginOverlap
  (params (OtherActor :type Actor%20Object%20Reference)))

(event EventTick
  (params (DeltaSeconds :type Float%20%28single-precision%29)))

(event EventInteractuar
  (if (Variables|Default|GetTieneBateria)
    (if (not (Variables|Default|GetEstaMoviendose))
      (CallFunction|IniciarRecorrido))
    (else
      (bind _asbp_third_person_character (Utilities|Casting|CastToBP_ThirdPersonCharacter (Game|GetPlayerCharacter 0)))
      (if (Variables|/Game/ThirdPerson/Blueprints/BP_ThirdPersonCharacter.BP_ThirdPersonCharacter_C|GetTieneBateria _asbp_third_person_character)
        (Variables|Default|SetTieneBateria true)
        (CallFunction|IniciarRecorrido)
        (else
          (Development|PrintString "No tengo energía.."))))))

(fn ConstructionScript)