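; BP_Valve is an interactable valve that turns a quarter turn with a sound when used.
; Clicking the actor calls Interact, while the OnValveInteracted event handles the response.
; That event stores the mesh's current yaw, plays the valve sound at the mesh's relative location, and restarts a timeline.
; The timeline's Giro curve lerps yaw 90 degrees onward, zeroing pitch and roll.
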(event Collision|EventActorBeginOverlap
  (params (OtherActor :type Actor%20Object%20Reference)))

(event EventTick
  (params (DeltaSeconds :type Float%20%28single-precision%29)))

(event MouseInput|EventActorOnClicked
  (params (ButtonPressed :type Key%20Structure :default "None"))
  (Class|ValveBase|Interact))

(event EventOnValveInteracted
  (params (NewAngle :type Float%20%28single-precision%29))
  (Variables|Default|SetRotacionInicial (.yaw (Variables|/Script/Engine.SceneComponent|GetRelativeRotation (Variables|Default|GetValveMesh))))
  (Audio|PlaySoundatLocation "/Game/Sounds/Sound_Valve.Sound_Valve" (Variables|/Script/Engine.SceneComponent|GetRelativeLocation (Variables|Default|GetValveMesh)) "0, 0, 0" 1.0 1.0 0.0 0 0 0 0)
  (bind _giro (Timeline|GiroTimeLine PlayFromStart)
    (:Update
      (Transformation|SetRelativeRotation (Variables|Default|GetValveMesh) (Math|Rotator|MakeRotator 0.0 0.0 (Math|Float|Lerp (Variables|Default|GetRotacionInicial) (- (Variables|Default|GetRotacionInicial) -9e+01) _giro)) false false))))

(fn ConstructionScript)