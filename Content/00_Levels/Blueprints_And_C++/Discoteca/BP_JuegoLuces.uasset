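; Light-timing minigame actor for the Discoteca level that rewards the player with a BP_LaboratorioLlave key.
; A self-restarting, Delay-driven round turns a spotlight green, then orange and red, while capsule overlaps track whether the player is inside.
; The player must be inside as green ends and outside shortly after red, otherwise the streak resets after a message.
; Three straight successes spawn the key and destroy the actor.
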(event OnComponentBeginOverlap(Capsule)
  (params (OverlappedComponent :type Primitive%20Component%20Object%20Reference) (OtherActor :type Actor%20Object%20Reference) (OtherComp :type Primitive%20Component%20Object%20Reference) (OtherBodyIndex :type Integer) (bFromSweep :type Boolean) (SweepResult :type Hit%20Result%20Structure%20%28by%20ref%29))
  (Utilities|Casting|CastToBP_ThirdPersonCharacter OtherActor)
  (Variables|Default|SetEstoyDentro true))

(event OnComponentEndOverlap(Capsule)
  (params (OverlappedComponent :type Primitive%20Component%20Object%20Reference) (OtherActor :type Actor%20Object%20Reference) (OtherComp :type Primitive%20Component%20Object%20Reference) (OtherBodyIndex :type Integer))
  (Utilities|Casting|CastToBP_ThirdPersonCharacter OtherActor)
  (Variables|Default|SetEstoyDentro false))

(event Custom|IniciarRonda
  (Rendering|Components|Light|SetLightColor (Variables|Default|GetSpotLight) "(R=0.000000,G=1.000000,B=0.000000,A=1.000000)" true)
  (Utilities|FlowControl|Delay 4.0)
  (if (Variables|Default|GetEstoyDentro)
    (Rendering|Components|Light|SetLightColor (Variables|Default|GetSpotLight) "(R=1.000000,G=0.298209,B=0.005113,A=1.000000)" true)
    (Utilities|FlowControl|Delay 1.5)
    (Rendering|Components|Light|SetLightColor (Variables|Default|GetSpotLight) "(R=1.000000,G=0.023006,B=0.000000,A=1.000000)" true)
    (Utilities|FlowControl|Delay 0.2)
    (if (Variables|Default|GetEstoyDentro)
      (Variables|Default|SetContadorAciertos 0)
      (Development|PrintString "LUZ ROJA, NO PUEDES ENTRAR")
      (Utilities|FlowControl|Delay 5.0)
      (CallFunction|IniciarRonda)
      (else
        (Variables|Default|SetContadorAciertos (+ (Variables|Default|GetContadorAciertos) 1))
        (if (>= (Variables|Default|GetContadorAciertos) 3)
          (Development|PrintString "GANASTE")
          (Game|SpawnActorfromClass "/Game/HUD/Pickups/BP_LaboratorioLlave.BP_LaboratorioLlave_C" (Transformation|GetActorTransform) "Undefined" "MultiplyWithRoot" 0 0)
          (Actor|DestroyActor)
          (else
            (Utilities|FlowControl|Delay 0.2)
            (CallFunction|IniciarRonda)))))
    (else
      (Variables|Default|SetContadorAciertos 0)
      (Development|PrintString "FALLASTE")
      (Utilities|FlowControl|Delay 5.0)
      (CallFunction|IniciarRonda))))

(event EventBeginPlay
  (CallFunction|IniciarRonda))

(fn ConstructionScript)