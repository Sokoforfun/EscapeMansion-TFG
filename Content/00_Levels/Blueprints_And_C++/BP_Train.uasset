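; Train actor that runs a locomotive and three wagons continuously along the Vía spline.
; Each Tick advances Distancia by Velocidad times delta time, wrapping it at the spline length.
; Each part takes its world location and rotation from the spline, with the locomotive's rotation offset by 180 degrees.
; Wagons trail at fixed distance offsets, which are not wrapped when they drop below zero.
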(event EventBeginPlay)

(event Collision|EventActorBeginOverlap
  (params (OtherActor :type Actor%20Object%20Reference)))

(event EventTick
  (params (DeltaSeconds :type Float%20%28single-precision%29))
  (bind _vía (Variables|Default|GetVía))
  (bind _vía_2 (Variables|Default|GetVía))
  (bind _vía_3 (Variables|Default|GetVía))
  (bind _vía_4 (Variables|Default|GetVía))
  (bind _output_get (Variables|Default|SetDistancia (Math|Float|%(Float) (+ (* DeltaSeconds (Variables|Default|GetVelocidad)) (Variables|Default|GetDistancia)) (Spline|GetSplineLength (Variables|Default|GetVía)))))
  (Transformation|SetWorldLocationAndRotation (Variables|Default|GetLocotomotora) (Spline|GetLocationatDistanceAlongSpline _vía_3 _output_get "World") (Math|Rotator|CombineRotators (Spline|GetRotationatDistanceAlongSpline _vía_3 _output_get "World") "0.000000,180.000000,0.000000") false false)
  (Transformation|SetWorldLocationAndRotation (Variables|Default|GetVagon1) (Spline|GetLocationatDistanceAlongSpline _vía_4 (- (Variables|Default|GetDistancia) 3e+02) "World") (Spline|GetRotationatDistanceAlongSpline _vía_4 (- (Variables|Default|GetDistancia) 3e+02) "World") false false)
  (Transformation|SetWorldLocationAndRotation (Variables|Default|GetVagon2) (Spline|GetLocationatDistanceAlongSpline _vía (- (Variables|Default|GetDistancia) 4e+02) "World") (Spline|GetRotationatDistanceAlongSpline _vía (- (Variables|Default|GetDistancia) 4e+02) "World") false false)
  (Transformation|SetWorldLocationAndRotation (Variables|Default|GetVagon3) (Spline|GetLocationatDistanceAlongSpline _vía_2 (- (Variables|Default|GetDistancia) 5e+02) "World") (Spline|GetRotationatDistanceAlongSpline _vía_2 (- (Variables|Default|GetDistancia) 5e+02) "World") false false))

(fn ConstructionScript)